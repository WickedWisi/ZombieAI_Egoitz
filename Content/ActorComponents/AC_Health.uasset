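; AC_Health is an actor component that tracks health for its owning actor and displays a floating health bar.
; On BeginPlay it adds a collision-free, screen-space WidgetComponent above the owner, holding a W_HealthBar initialized with the current health and owning actor.
; TakeDamage subtracts from Health without clamping, fires OnDamageTaken, and fires OnDeath whenever the result is zero or below.
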(event `self.ReceiveBeginPlay`
  (bind _returnvalue (`|AddComponentByClass` (`self.GetOwner`) "/Script/UMG.WidgetComponent" false (`KismetMathLibrary.MakeTransform` (0.0 0.0 100.0))))
  (`WidgetComponent.SetDrawSize` _returnvalue (150.0 10.0))
  (`WidgetComponent.SetWidgetSpace` _returnvalue "Screen")
  (`PrimitiveComponent.SetCollisionEnabled` _returnvalue "NoCollision")
  (bind _returnvalue_2 (`|CreateWidget` "/Game/ThirdPerson/Blueprints/W_HealthBar.W_HealthBar_C" null (`self.Health`) (`self.GetOwner`)))
  (`WidgetComponent.SetWidget` _returnvalue _returnvalue_2))

(fn `TakeDamage`
  (params (`Damage Amount` :type "Float (double-precision)" :default 50.0))
  (bind _output_get (set `self.Health` (- (`self.Health`) `Damage Amount`)))
  (`self.OnDamageTaken`)
  (if (<= _output_get 0.0)
    (`self.OnDeath`)))